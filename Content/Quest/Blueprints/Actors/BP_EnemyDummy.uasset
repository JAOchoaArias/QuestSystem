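; BP_EnemyDummy is a damageable target dummy that reports a quest objective when killed.
; It accepts damage only from BP_TopDownCharacter and updates a WBP_EnemyHealthBar widget.
; Health is set to the larger of current health and damage, not reduced by subtraction.
; At zero health it calls ReportObjective, destroying itself on success or reviving at full health otherwise.
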(event `self.ReceiveBeginPlay`
  (set `self.CurrentHealth` (`self.MaxHealth`)))

(event `self.ReceiveAnyDamage`
  (params (Damage :type "Float (single-precision)") (DamageType :type "DamageType Object Reference") (InstigatedBy :type "Controller Object Reference") (DamageCauser :type "Actor Object Reference"))
  (if (not (`self.IsDead`))
    (cast `/Game/TopDown/Blueprints/BP_TopDownCharacter` DamageCauser)
    (bind _output_get (set `self.CurrentHealth` (`KismetMathLibrary.FMax` (`self.CurrentHealth`) Damage)))
    (bind _aswbp_enemy_health_bar (cast `/Game/Quest/Blueprints/UI/WBP_EnemyHealthBar` (`WidgetComponent.GetUserWidgetObject` (`self.HealthBarComponent`))))
    (`/Game/Quest/Blueprints/UI/WBP_EnemyHealthBar.SetHealthPercent}` _aswbp_enemy_health_bar (/ _output_get (`self.MaxHealth`)))
    (if (<= _output_get 0.0)
      (set `self.IsDead` true)
      (bind _succes (`self.ReportObjective`))
      (if _succes
        (`self.K2_DestroyActor`)
        (else
          (set `self.IsDead` false)
          (set `self.CurrentHealth` (`self.MaxHealth`))
          (`/Game/Quest/Blueprints/UI/WBP_EnemyHealthBar.SetHealthPercent}` _aswbp_enemy_health_bar 1.0))))))

(fn `UserConstructionScript`
  (`parent.UserConstructionScript`))