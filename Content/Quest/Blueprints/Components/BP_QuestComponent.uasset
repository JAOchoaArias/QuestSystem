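; Quest component that stores runtime quests created from quest definitions and tracks their objective progress.
; AddQuest rejects duplicate IDs, while objective events from BP_QuestGameState advance objectives with matching type and target in active quests, capped at the required amount.
; Struct copies are written back into ActiveQuests, and dispatchers announce start, progress and completion.
; The completion check after each update always receives index 0, not the updated quest's index.
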(event `self.ReceiveBeginPlay`
  (bind _asbp_quest_game_state (cast `/Game/Quest/Blueprints/GameState/BP_QuestGameState` (`GameplayStatics.GetGameState`)))
  (add `/Game/Quest/Blueprints/GameState/BP_QuestGameState.OnGameplayObjectiveEvent` _asbp_quest_game_state (delegate `HandleGameplayObjective`)))

(event `HandleGameplayObjective`
  (params (ObjectiveType :type "/Game/Quest/Blueprints/Enums/EQuestObjectiveType Enum" :default "NewEnumerator0") (TargetID :type Name) (Amount :type Integer))
  (for (_array_element _array_index) (`self.ActiveQuests`)
    (bind (_questid _questdefinition _objectives _isactive _iscompleted) (break `/Game/Quest/Blueprints/Structs/ST_QuestRuntime` _array_element))
    (if (and _isactive (not _iscompleted))
      (for (_array_element_2 _array_index_2) _objectives
        (bind (_obectiveid _objectivetype _targetid) (break `/Game/Quest/Blueprints/Structs/ST_QuestObjective` _array_element_2))
        (if (and (== _targetid TargetID) (`|EnumEquality` _objectivetype ObjectiveType))
          (`self.UpdateObjectiveProgress` _array_index _array_index_2 Amount))))))

(fn `AddQuest`
  (params (QuestDefinition :type "/Game/Quest/Blueprints/Data/PDA_QuestDefinition Object Reference"))
  (bind _questid (`/Game/Quest/Blueprints/Data/PDA_QuestDefinition.QuestID` QuestDefinition))
  (bind _st_questruntime (make `/Game/Quest/Blueprints/Structs/ST_QuestRuntime` _questid QuestDefinition (`/Game/Quest/Blueprints/Data/PDA_QuestDefinition.Objectives` QuestDefinition) true))
  (`/Engine/EditorBlueprintResources/StandardMacros.IsValid` QuestDefinition
    (:`Is Valid`
      (bind _found (`self.FindQuestByID` _questid))
      (if (not _found)
        (`KismetArrayLibrary.Array_Add` (`self.ActiveQuests`) _st_questruntime)
        (`self.OnQuestStarted` _st_questruntime)))))

(fn `CheckQuestCompleted`
  (params (QuestIndex :type Integer))
  (locals (AllCompleted :type Boolean) (LocalQuest :type "/Game/Quest/Blueprints/Structs/ST_QuestRuntime Structure"))
  (bind _activequests (`self.ActiveQuests`))
  (bind _allcompleted (`local.AllCompleted`))
  (bind _output_get (set `local.LocalQuest` (`|GetArrayItem` _activequests QuestIndex)))
  (set `local.AllCompleted` true)
  (for _array_element (`.Objectives_13_851EA1054004708867B2F086A61972BE` (break `/Game/Quest/Blueprints/Structs/ST_QuestRuntime` _output_get))
    (bind (_obectiveid _objectivetype _targetid _requiredamount _currentamount) (break `/Game/Quest/Blueprints/Structs/ST_QuestObjective` _array_element))
    (if (not (>= _currentamount _requiredamount))
      (set `local.AllCompleted` false)))
  (if _allcompleted
    (setmembers `/Game/Quest/Blueprints/Structs/ST_QuestRuntime` :`StructRef` _output_get :`IsActive` false :`IsCompleted` true)
    (`KismetArrayLibrary.Array_Set` _activequests QuestIndex _output_get))
  (`self.OnQuestProgressChanged` _output_get)
  (if _allcompleted
    (`self.OnQuestCompleted` _output_get)))

(fn `FindQuestByID`
  (params (QuestID :type Name))
  (returns (Found :type Boolean) (QuestData :type "/Game/Quest/Blueprints/Structs/ST_QuestRuntime Structure") (QuestIndex :type Integer))
  (for (_array_element _array_index) (`self.ActiveQuests`)
    (if (== (`.QuestID_10_68464FA642884E6E45B6CD9447016617` (break `/Game/Quest/Blueprints/Structs/ST_QuestRuntime` _array_element)) QuestID)
      (return true _array_element _array_index)))
  (return false (struct) -1))

(fn `UpdateObjectiveProgress`
  (params (QuestIndex :type Integer) (ObjectiveIndex :type Integer) (Amount :type Integer))
  (locals (LocalObjective :type "/Game/Quest/Blueprints/Structs/ST_QuestObjective Structure") (LocalObjectives :type "Array of /Game/Quest/Blueprints/Structs/ST_QuestObjective Structure") (LocalQuest :type "/Game/Quest/Blueprints/Structs/ST_QuestRuntime Structure") (NewAmount :type Integer))
  (bind _activequests (`self.ActiveQuests`))
  (bind _output_get (set `local.LocalQuest` (`|GetArrayItem` _activequests QuestIndex)))
  (bind _output_get_2 (set `local.LocalObjectives` (`.Objectives_13_851EA1054004708867B2F086A61972BE` (break `/Game/Quest/Blueprints/Structs/ST_QuestRuntime` _output_get))))
  (bind _output_get_3 (set `local.LocalObjective` (`|GetArrayItem` _output_get_2 ObjectiveIndex)))
  (bind (_obectiveid _objectivetype _targetid _requiredamount _currentamount) (break `/Game/Quest/Blueprints/Structs/ST_QuestObjective` _output_get_3))
  (bind _output_get_4 (set `local.NewAmount` (`KismetMathLibrary.Min` (+ _currentamount Amount) _requiredamount)))
  (setmembers `/Game/Quest/Blueprints/Structs/ST_QuestObjective` :`StructRef` _output_get_3 :`CurrentAmount` _output_get_4)
  (`KismetArrayLibrary.Array_Set` _output_get_2 ObjectiveIndex _output_get_3)
  (setmembers `/Game/Quest/Blueprints/Structs/ST_QuestRuntime` :`StructRef` _output_get :`Objectives` _output_get_2)
  (`KismetArrayLibrary.Array_Set` _activequests QuestIndex _output_get)
  (`self.CheckQuestCompleted` 0))